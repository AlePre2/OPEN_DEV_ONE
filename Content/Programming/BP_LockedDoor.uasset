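; Door that swings open for the player once every NPC in its list has been interacted with.
; On BeginPlay it binds to each NPC's first-interaction event and counts the callbacks.
; When the first-person character overlaps the box with the count met, a one-shot delayed timeline rotates the root's yaw toward DoorRotation, lerping from the current yaw each update.
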(event OnComponentBeginOverlap(Box)
  (params (OverlappedComponent :type Primitive%20Component%20Object%20Reference) (OtherActor :type Actor%20Object%20Reference) (OtherComp :type Primitive%20Component%20Object%20Reference) (OtherBodyIndex :type Integer) (bFromSweep :type Boolean) (SweepResult :type Hit%20Result%20Structure%20%28by%20ref%29))
  (Utilities|Casting|CastToBP_FirstPersonCharacter OtherActor)
  (if (>= (Variables|Default|GetNpcInteractionAmount) (Utilities|Array|Length (Variables|Default|GetNpcsList)))
    (Utilities|FlowControl|DoOnce false
      (:Completed
        (Utilities|FlowControl|Delay 0.4)
        (bind _door (Timeline|doorAnimation Play)
          (:Update
            (Transformation|SetRelativeRotation (Variables|Default|GetDefaultSceneRoot) (Math|Rotator|MakeRotator 0.0 0.0 (Math|Float|Lerp (.yaw (Variables|/Script/Engine.SceneComponent|GetRelativeRotation (Variables|Default|GetDefaultSceneRoot))) (Variables|Default|GetdoorRotation) _door)) false false)))))))

(event Custom|HasInteractedWithNpc
  (Variables|Default|SetNpcInteractionAmount (+ (Variables|Default|GetNpcInteractionAmount) 1)))

(event EventBeginPlay
  (for _array_element (Variables|Default|GetNpcsList)
    (EventDispatchers|BindEventtoFirstInteractionwithNpc _array_element (delegate Custom|HasInteractedWithNpc))))

(event Collision|EventActorBeginOverlap
  (params (OtherActor :type Actor%20Object%20Reference)))

(event EventTick
  (params (DeltaSeconds :type Float%20%28single-precision%29)))

(fn ConstructionScript)